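; Automatic sliding glass door Blueprint that opens on overlap with its collision component and closes when the overlap ends.
; The Construction Script caches the world locations of the two door meshes as DoorL and DoorR.
; A timeline track is subtracted from one and added to the other, sliding the panels in opposite directions, and plays in reverse to close them.
; Overlaps are not filtered by actor.
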(event OnComponentBeginOverlap(CollisionComp)
  (params (OverlappedComponent :type Primitive%20Component%20Object%20Reference) (OtherActor :type Actor%20Object%20Reference) (OtherComp :type Primitive%20Component%20Object%20Reference) (OtherBodyIndex :type Integer) (bFromSweep :type Boolean) (SweepResult :type Hit%20Result%20Structure%20%28by%20ref%29))
  (bind _newtrack_0 (Timeline|Timeline_0 Play)
    (:Update
      (Transformation|SetWorldLocation (Variables|Default|GetStaticMeshComponent0) (- (Variables|Default|GetDoor_L) _newtrack_0) false false)
      (Transformation|SetWorldLocation (Variables|Default|GetStaticMeshComponent01) (+ _newtrack_0 (Variables|Default|GetDoor_R)) false false))))

(event OnComponentEndOverlap(CollisionComp)
  (params (OverlappedComponent :type Primitive%20Component%20Object%20Reference) (OtherActor :type Actor%20Object%20Reference) (OtherComp :type Primitive%20Component%20Object%20Reference) (OtherBodyIndex :type Integer))
  (bind _newtrack_0 (Timeline|Timeline_0 Reverse)
    (:Update
      (Transformation|SetWorldLocation (Variables|Default|GetStaticMeshComponent0) (- (Variables|Default|GetDoor_L) _newtrack_0) false false)
      (Transformation|SetWorldLocation (Variables|Default|GetStaticMeshComponent01) (+ _newtrack_0 (Variables|Default|GetDoor_R)) false false))))

(event EventBeginPlay)

(event Collision|EventActorBeginOverlap
  (params (OtherActor :type Actor%20Object%20Reference)))

(event EventTick
  (params (DeltaSeconds :type Float%20%28single-precision%29)))

(fn ConstructionScript
  (Variables|Default|SetDoor_L (Transformation|GetWorldLocation (Variables|Default|GetStaticMeshComponent0)))
  (Variables|Default|SetDoor_R (Transformation|GetWorldLocation (Variables|Default|GetStaticMeshComponent01))))